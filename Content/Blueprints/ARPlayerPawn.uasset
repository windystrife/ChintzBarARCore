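; AR player pawn that places one chintz fish, gold fish or teleport portal on a detected plane where the screen is touched.
; IsAndroid switches between ARCore and ARKit hit tests and spawn logic, with main-widget state choosing what appears.
; Tick updates tracking prompts and gold-fish UI, spawns ARCore plane actors, and binds two-way portal overlap teleports.
; The pawn's own GPS and weekend gold-fish check is disconnected.
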(fn `CachePlatform`
  ;[1 1 1] Cache platform that we're running on for switching on platform-specific functionality
  (bind _returnvalue (`GameplayStatics.GetPlatformName`))
  (bind _output_get (set `self.bIsAndroid` (== _returnvalue "Android")))
  (`KismetSystemLibrary.PrintString` _returnvalue)
  (`KismetSystemLibrary.PrintString` (`KismetStringLibrary.Conv_BoolToString` _output_get)))

(fn `DetermineTrackingQuality`
  (returns (Tracking :type "EARTrackingQuality Enum"))
  (locals (TrackingQuality :type "EARTrackingQuality Enum" :default "NotAvailable"))
  ;[1 1 1] If we haven't found any planes yet, downgrade the tracking quality by 1 notch.
  (bind _returnvalue (`ARBlueprintFunctionLibrary.GetTrackingQuality`))
  (bind _output_get (set `local.TrackingQuality` _returnvalue))
  (bind _returnvalue_2 (select `bool` (>= (`self.numPlanesDetected`) 1) :`false` (select `EARTrackingQuality` _output_get :`NotAvailable` "NotAvailable" :`Limited` "Limited" :`Normal` "Limited" :!type "EARTrackingQuality Enum") :`true` _output_get))
  (set `self.trackquality_public` _returnvalue_2)
  (return _returnvalue_2))

(fn `DisplayDebugTrackingInfo`
  ;[1 1 1] Display Debug Tracking Info
  (`KismetSystemLibrary.PrintString` (`KismetStringLibrary.Conv_TransformToString` (`SceneComponent.K2_GetComponentToWorld` (`PlayerCameraManager.TransformComponent` (`GameplayStatics.GetPlayerCameraManager` 0)))) true false (struct :`R` 0.081168 :`G` 1.0 :`B` 0.218801 :`A` 1.0) 0.0)
  (bind _tracking (`self.DetermineTrackingQuality`))
  (`KismetSystemLibrary.PrintString` (`KismetStringLibrary.Concat_StrStr` "[ " (`|GetEnumeratorNameAsString` _tracking) " ]") true false (select `EARTrackingQuality` _tracking :`NotAvailable` (struct :`R` 1.0 :`B` 0.158961 :`A` 1.0) :`Limited` (struct :`R` 1.0 :`G` 0.226966 :`A` 1.0) :`Normal` (struct :`R` 0.283149 :`G` 1.0 :`A` 1.0) :!type "LinearColor Structure") 0.0))

(fn `DoHitTestForARCORE`
  (params (Player :type "PlayerController Object Reference") (InputPin :type "Vector2D Structure"))
  (returns (Success :type Boolean) (SpawnTransform :type "Transform Structure") (Plane :type "GoogleARCorePlane Object Reference") (SpawnPortal :type "Transform Structure"))
  (bind (_worldposition _worlddirection) (`GameplayStatics.DeprojectScreenToWorld` Player InputPin))
  (bind (_impactpoint _impactnormal _outplaneobject _returnvalue) (`GoogleARCoreSessionFunctionLibrary.LineTraceSingleOnPlanes` _worldposition (+ _worldposition (* _worlddirection 10000.0))))
  (if _returnvalue
    (`KismetSystemLibrary.PrintString` (`KismetStringLibrary.Concat_StrStr` "HIT from :  " (`KismetStringLibrary.Conv_Vector2dToString` InputPin)) true true (struct :`R` 0.7074 :`G` 1.0 :`A` 1.0))
    (bind _returnvalue_2 (`KismetMathLibrary.MakeTransform` _impactpoint))
    (`KismetSystemLibrary.PrintString` (`KismetStringLibrary.Conv_TransformToString` _returnvalue_2) true true (struct :`R` 1.0 :`G` 0.96541 :`A` 1.0))
    (bind _location (.location _returnvalue_2))
    (bind _scale (.scale _returnvalue_2))
    (bind _roll (.roll (`KismetMathLibrary.FindLookAtRotation` _impactpoint (+ _impactpoint (`KismetMathLibrary.Normal` (* _worlddirection (1.0 1.0 0.0)))))))
    (bind _pitch (.pitch (`KismetMathLibrary.FindLookAtRotation` _impactpoint (+ _impactpoint (`KismetMathLibrary.Normal` (* _worlddirection (1.0 1.0 0.0)))))))
    (bind _yaw (.yaw (`KismetMathLibrary.FindLookAtRotation` _impactpoint (+ _impactpoint (`KismetMathLibrary.Normal` (* _worlddirection (1.0 1.0 0.0)))))))
    (return true (`KismetMathLibrary.MakeTransform` _location (`KismetMathLibrary.MakeRotator` _roll _pitch (- _yaw -90.0)) _scale) _outplaneobject (`KismetMathLibrary.MakeTransform` _location (`KismetMathLibrary.MakeRotator` _roll _pitch (+ _yaw 180.0)) _scale))
    (else
      (return false (struct) null))))

(fn `DoHitTestForARKIT`
  (params (InputPin :type "Vector2D Structure") (Player :type "PlayerController Object Reference"))
  (returns (Success :type Boolean) (SpawnTransform :type "Transform Structure") (SpawnPortal :type "Transform Structure"))
  (bind (_outresults _returnvalue) (`AppleARKitBlueprintLibrary.HitTestAtScreenPosition_TrackingSpace` InputPin "ExistingPlane"))
  (if _returnvalue
    (bind (_type _distance _transform) (break `AppleARKitHitTestResult` (`|GetArrayItem` _outresults)))
    (`KismetSystemLibrary.PrintString` (`KismetStringLibrary.Concat_StrStr` "HIT from :  " (`KismetStringLibrary.Conv_Vector2dToString` InputPin) " Distance : " (`KismetStringLibrary.Conv_DoubleToString` _distance)) true true (struct :`R` 0.7074 :`G` 1.0 :`A` 1.0))
    (`KismetSystemLibrary.PrintString` (`KismetStringLibrary.Conv_TransformToString` _transform) true true (struct :`R` 1.0 :`G` 0.96541 :`A` 1.0))
    (bind _location (.location _transform))
    (bind _scale (.scale _transform))
    (bind _returnvalue_2 (`KismetMathLibrary.FindLookAtRotation` _location (+ _location (`KismetMathLibrary.Normal` (* (`.WorldDirection` (`GameplayStatics.DeprojectScreenToWorld` Player InputPin)) (1.0 1.0 0.0))))))
    (return true (`KismetMathLibrary.MakeTransform` _location (`KismetMathLibrary.MakeRotator` (.roll _returnvalue_2) (.pitch _returnvalue_2) (- (.yaw _returnvalue_2) -90.0)) _scale) (`KismetMathLibrary.MakeTransform` _location (`KismetMathLibrary.MakeRotator` (.roll _returnvalue_2) (.pitch _returnvalue_2) (+ (.yaw _returnvalue_2) 180.0)) _scale))
    (else
      (return false))))

(fn `FindPlanesForARCORE`
  (bind _outarcoreplanelist (`GoogleARCoreFrameFunctionLibrary.GetAllPlanes`))
  (bind _returnvalue (`KismetArrayLibrary.Array_Length` _outarcoreplanelist))
  (`KismetSystemLibrary.PrintString` (`KismetStringLibrary.Conv_IntToString` _returnvalue) true false (struct :`G` 0.66 :`B` 1.0 :`A` 1.0) 0.0)
  (set `self.numPlanesDetected` _returnvalue))

(fn `FishGoldSpawn?`
  (returns (InLocation :type Boolean) (RightTime :type Boolean) (SpawnGoldFish :type Boolean))
  (locals (DateTime :type "DateTime Structure"))
  (bind _latitude (`self.Latitude`))
  (bind _longitude (`self.Longitude`))
  (bind (_year _month _day _hour) (`KismetMathLibrary.BreakDateTime` (`local.DateTime`)))
  (bind _returnvalue (and (and (<= _latitude 50.459433) (>= _latitude 50.45885)) (and (<= _longitude -4.377846) (>= _longitude -4.377999))))
  (set `local.DateTime` (`KismetMathLibrary.Now`))
  (bind _returnvalue_2 (`WeekDay.WeekDay` _year _month _day))
  (if (and (or (== _returnvalue_2 7) (== _returnvalue_2 1)) (and (<= _hour 24) (> _hour 12)))
    (if _returnvalue
      (return true true true)
      (else
        (return false true false)))
    (elif _returnvalue
      (return true false false)
      (else
        (return false false false)))))

(fn `UPdateARCorePlaneActor`
  ;[1 1 1] Loop through all the plane objects
  (bind _outarcoreplanelist (`GoogleARCoreFrameFunctionLibrary.GetAllPlanes`))
  (for _array_element _outarcoreplanelist
    (`|ExecutionSequence`
      (:`then_0`
        (bind _output_get (set `self.ARPlane Object` _array_element))
        (set `self.PlaneId` (`GoogleARCorePlane.GetPlaneId` _output_get)))
      (:`then_1`
        ;[1 1 1] Spawn a new Plane Actor if it hasn't been created for a specific PlaneId, or the Plane Actor has been destroyed due to the Plane object has stopped tracking or subsumed
        (if true
          (if (not (`KismetSystemLibrary.IsValid` (`BlueprintMapLibrary.Map_Find` (`self.PlaneActorMap`) (`self.PlaneId`))))
            (`BlueprintMapLibrary.Map_Remove` (`self.PlaneActorMap`) (`self.PlaneId`))
            (bind _returnvalue (`|SpawnActorFromClass` "/Game/Blueprints/ARCorePlaneActor.ARCorePlaneActor_C" (`KismetMathLibrary.MakeTransform` (0.0 0.0 0.0)) "Undefined" "OverrideRootScale" null null :!label _label))
            (set `ARPlaneActor.ARCorePlaneObject` (`self.ARPlane Object`) _returnvalue)
            (`BlueprintMapLibrary.Map_Add` (`self.PlaneActorMap`) (`self.PlaneId`) _returnvalue))
          (else
            (goto _label)))))))

(fn `UserConstructionScript`)