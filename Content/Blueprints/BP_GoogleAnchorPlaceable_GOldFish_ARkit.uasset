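; Placeable AR actor, named as a goldfish Google anchor for ARKit, whose event graph and construction script currently run no logic.
; Unconnected nodes would cache a child GoogleARCoreAnchorActor, start location services, store latitude and longitude, and print debug status.
; GetDayOfWeek computes a 1–7 weekday from day, month and year with a Zeller-style formula, treating January and February as the previous year's months.
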(event `self.ReceiveBeginPlay`)

(event `self.ReceiveTick`
  (params (DeltaSeconds :type "Float (single-precision)")))

(fn `GetDayOfWeek`
  (params (Day :type Integer) (Month :type Integer) (Year :type Integer))
  (returns (DayOfWeek :type Integer))
  (locals (YearTemp :type Integer) (DayTemp :type Integer) (MonthTemp :type Integer) (DayOfTheWeek :type Integer))
  (set `local.DayTemp` Day)
  (set `local.MonthTemp` Month)
  (set `local.YearTemp` Year)
  (if (< Month 3)
    (set `local.MonthTemp` (+ (`local.MonthTemp`) 12))
    (set `local.YearTemp` (- (`local.YearTemp`) 1)))
  (bind _output_get (set `local.DayOfTheWeek` (+ (mod (`KismetMathLibrary.Abs_Int` (+ (`local.DayTemp`) (`KismetMathLibrary.FTrunc` (* (`local.MonthTemp`) 2.0)) (`KismetMathLibrary.FTrunc` (/ (* (+ (`local.MonthTemp`) 1) 3.0) 5.0)) (`local.YearTemp`) (/ (`local.YearTemp`) 4))) 7) 1)))
  (return _output_get))

(fn `UserConstructionScript`)